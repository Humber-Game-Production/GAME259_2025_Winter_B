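; Interactable numpad actor for the code puzzle that opens a Numpad UI when the player interacts within range.
; Box overlap toggles a prompt widget and, for BP_ThirdPersonCharacter, enables or disables the actor's input.
; Interact flip-flops between showing the Numpad with mouse cursor and a shared close path, also run on leaving the box.
; Closing removes all widgets and restores game-only input, without resetting the flip-flop.
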(event `self.Box.OnComponentBeginOverlap`
  (params (OverlappedComponent :type "PrimitiveComponent Object Reference") (OtherActor :type "Actor Object Reference") (OtherComp :type "PrimitiveComponent Object Reference") (OtherBodyIndex :type Integer) (bFromSweep :type Boolean) (SweepResult :type "HitResult Structure (by ref)"))
  ; E to Interact Prompt
  (`SceneComponent.SetVisibility` (`self.Widget`) true false)
  (cast `/Game/ThirdPerson/Blueprints/BP_ThirdPersonCharacter` OtherActor)
  (`self.EnableInput` (`GameplayStatics.GetPlayerController` 0)))

(event `self.Box.OnComponentEndOverlap`
  (params (OverlappedComponent :type "PrimitiveComponent Object Reference") (OtherActor :type "Actor Object Reference") (OtherComp :type "PrimitiveComponent Object Reference") (OtherBodyIndex :type Integer))
  (bind _returnvalue (`GameplayStatics.GetPlayerController` 0))
  ; E to Interact Prompt
  (`SceneComponent.SetVisibility` (`self.Widget`) false false)
  (cast `/Game/ThirdPerson/Blueprints/BP_ThirdPersonCharacter` OtherActor)
  (`self.DisableInput` (`GameplayStatics.GetPlayerController` 0))
  ; Shows Numpad upon interaction, disables input and shows mouse
  (`WidgetLayoutLibrary.RemoveAllWidgets` :!label _label)
  (`WidgetBlueprintLibrary.SetInputMode_GameOnly` _returnvalue)
  (set `PlayerController.bShowMouseCursor` false _returnvalue))

(event `/Game/ButtonPuzzle/InteractInterface.Interact`
  (params (Player :type Boolean))
  (bind _returnvalue (`GameplayStatics.GetPlayerController` 0))
  ; Shows Numpad upon interaction, disables input and shows mouse
  (`/Engine/EditorBlueprintResources/StandardMacros.FlipFlop`
    (:`A`
      (bind _returnvalue_2 (`|CreateWidget` "/Game/CodePuzzle/Numpad.Numpad_C"))
      (`UserWidget.AddToViewport` _returnvalue_2 0)
      (`WidgetBlueprintLibrary.SetInputMode_GameAndUIEx` _returnvalue _returnvalue_2)
      (set `PlayerController.bShowMouseCursor` true _returnvalue))
    (:`B`
      (goto _label))))

(fn `UserConstructionScript`)