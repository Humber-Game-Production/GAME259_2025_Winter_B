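; Main menu game mode that manages navigation between the main menu, controller and credits screens.
; On BeginPlay it creates all three widgets once, binds their event dispatchers to its handlers and shows the main menu.
; Each handler swaps screens by removing the current widget from its parent and adding the requested one to the viewport, so the cached instances are reused.
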(event `self.ReceiveBeginPlay`
  ;[0.05729 0.05729 0.05729] Creation of main menu widget
  (bind _returnvalue (`|CreateWidget` "/Game/BTeamCONTENTfolder/Blueprints/UI_BP/WB_MainMenu.WB_MainMenu_C"))
  (bind _output_get (set `self.WBR_MainMenu` _returnvalue))
  (bind _returnvalue_2 (`|CreateWidget` "/Game/BTeamCONTENTfolder/Blueprints/UI_BP/WB_Controller.WB_Controller_C"))
  (bind _output_get_2 (set `self.WBR_Controller` _returnvalue_2))
  (bind _returnvalue_3 (`|CreateWidget` "/Game/BTeamCONTENTfolder/Blueprints/UI_BP/WB_Credits.WB_Credits_C"))
  (bind _output_get_3 (set `self.WBR_Credits` _returnvalue_3))
  (add `/Game/BTeamCONTENTfolder/Blueprints/UI_BP/WB_MainMenu.ED_OpenControllerWidget` _output_get (delegate `OpenControllerWindow`))
  (add `/Game/BTeamCONTENTfolder/Blueprints/UI_BP/WB_Controller.ED_OpenMainMenu` _output_get_2 (delegate `OpenMainMenu`))
  (add `/Game/BTeamCONTENTfolder/Blueprints/UI_BP/WB_Credits.ED_OpenMainMenu` _output_get_3 (delegate `OpenMainMenu`))
  (add `/Game/BTeamCONTENTfolder/Blueprints/UI_BP/WB_MainMenu.ED_OpenCreditsWidget` _output_get (delegate `OpenCreditsMenu`))
  (`UserWidget.AddToViewport` _output_get 0))

(event `OpenControllerWindow`
  (`Widget.RemoveFromParent` (`self.WBR_MainMenu`))
  (`UserWidget.AddToViewport` (`self.WBR_Controller`) 0))

(event `OpenMainMenu`
  (`Widget.RemoveFromParent` (`self.WBR_Credits`))
  (`Widget.RemoveFromParent` (`self.WBR_Controller`))
  (`UserWidget.AddToViewport` (`self.WBR_MainMenu`) 0))

(event `OpenCreditsMenu`
  (`Widget.RemoveFromParent` (`self.WBR_MainMenu`))
  (`UserWidget.AddToViewport` (`self.WBR_Credits`) 0))

(fn `UserConstructionScript`)