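; HUD component that shows the puzzle legend and opens the pause menu.
; On BeginPlay it creates the legend widget for the first player controller and adds it to the viewport, with events to show or remove it.
; Pressing P creates a new pause widget, switches input to Game and UI, shows the cursor and pauses the game, with no unpause logic here.
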(event `self.ReceiveBeginPlay`
  (bind _returnvalue (`|CreateWidget` "/Game/BTeamCONTENTfolder/Blueprints/UI_BP/WB_PuzzleLegend.WB_PuzzleLegend_C" (`GameplayStatics.GetPlayerController` 0)))
  (set `self.WBR_HUD` _returnvalue)
  (`self.Open Legend`))

(event `Open Legend`
  (`UserWidget.AddToViewport` (`self.WBR_HUD`) 0))

(event `Close Legend`
  (`Widget.RemoveFromParent` (`self.WBR_HUD`)))

(event `Key|P`
  (params (Key :type "Key Structure"))
  (bind _returnvalue (`GameplayStatics.GetPlayerController` 0))
  (:`Pressed`
    (bind _returnvalue_2 (`|CreateWidget` "/Game/BTeamCONTENTfolder/Blueprints/UI_BP/WB_Pause.WB_Pause_C" _returnvalue))
    (bind _output_get (set `self.WBR_PauseMenu` _returnvalue_2))
    (`UserWidget.AddToViewport` _output_get 0)
    (`WidgetBlueprintLibrary.SetInputMode_GameAndUIEx` _returnvalue _output_get)
    (set `PlayerController.bShowMouseCursor` true _returnvalue)
    (`GameplayStatics.SetGamePaused` true)))