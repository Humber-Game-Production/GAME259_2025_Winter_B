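; Actor that shows a controller-disconnect overlay when the connected input device count is anything other than four.
; It binds to the GameInstance's input device connection change event on BeginPlay and unbinds on Destroyed.
; Each event adjusts a running count, removing the widget at exactly four and otherwise adding it to the viewport.
; The WB_ControllerDisconnect widget is created lazily for player controller 0 and reused.
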(event `self.ReceiveBeginPlay`
  (add `GameInstance.OnInputDeviceConnectionChange` (`GameplayStatics.GetGameInstance`) (delegate `Event Input Device Connection Change`)))

(event `self.ReceiveDestroyed`
  (remove `GameInstance.OnInputDeviceConnectionChange` (`GameplayStatics.GetGameInstance`) (delegate `Event Input Device Connection Change`)))

(event `Event Input Device Connection Change`
  (params (NewConnectionState :type "EInputDeviceConnectionState Enum" :default "Invalid") (PlatformUserId :type "PlatformUserId Structure") (InputDeviceId :type "InputDeviceId Structure"))
  (bind _connecteddevicecount (`self.ConnectedDeviceCount`))
  (bind _disconnecteddevicewidget (`self.DisconnectedDeviceWidget`))
  (bind _returnvalue (`KismetSystemLibrary.IsValid` _disconnecteddevicewidget))
  (if (`|EnumEquality` NewConnectionState "Connected")
    (`/Engine/EditorBlueprintResources/StandardMacros.IncrementInt` _connecteddevicecount
      (:`  `
        _))
    (else
      (`/Engine/EditorBlueprintResources/StandardMacros.DecrementInt` _connecteddevicecount
        (:`  `
          _))))
  (if (== _connecteddevicecount 4)
    (if _returnvalue
      (`Widget.RemoveFromParent` _disconnecteddevicewidget))
    (else
      (if (not _returnvalue)
        (bind _returnvalue_2 (`|CreateWidget` "/Game/BTeamCONTENTfolder/Blueprints/UI_BP/WB_ControllerDisconnect.WB_ControllerDisconnect_C" (`GameplayStatics.GetPlayerControllerFromID` 0)))
        (bind _output_get (set `self.DisconnectedDeviceWidget` _returnvalue_2)))
      (`UserWidget.AddToViewport` _output_get 0))))

(fn `UserConstructionScript`)